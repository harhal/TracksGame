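; Main gameplay PlayerController that manages UI screens and player input.
; On BeginPlay it adds the achievement widget and sets game-only input; EndGame shows the end screen with the win flag and a highscore check.
; Pause freezes the game and opens a pause widget, or loads MainMenu when no pawn is possessed.
; Axis and Jump inputs are forwarded to the controlled pawn after validity checks.
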(event `self.ReceiveBeginPlay`
  ;[1 1 1] UI Inicializer
  (bind _returnvalue (`|CreateWidget` "/Game/UI/AchivementWidget.AchivementWidget_C" self))
  (`UserWidget.AddToViewport` _returnvalue 0)
  (set `self.AchivementWidget` _returnvalue)
  (`WidgetBlueprintLibrary.SetInputMode_GameOnly` self)
  (set `self.bShowMouseCursor` false))

(event `EndGame`
  (params (Win :type Boolean))
  ;[1 1 1] End Game
  (bind _returnvalue (`|CreateWidget` "/Game/UI/EndGameUI.EndGameUI_C" self))
  (set `/Game/UI/EndGameUI.IsWin` Win _returnvalue)
  (`/Game/UI/EndGameUI.CheckHighscore` _returnvalue)
  (`UserWidget.AddToViewport` _returnvalue 0)
  (`WidgetBlueprintLibrary.SetInputMode_UIOnlyEx` self _returnvalue)
  (set `self.bShowMouseCursor` true))

(event `InputAction|Pause`
  (params (Key :type "Key Structure"))
  ;[1 1 1] Pause
  (:`Pressed`
    (`/Engine/EditorBlueprintResources/StandardMacros.IsValid` (`self.K2_GetPawn`)
      (:`Is Valid`
        (`GameplayStatics.SetGamePaused` true)
        (bind _returnvalue (`|CreateWidget` "/Game/UI/PauseWidget.PauseWidget_C"))
        (`UserWidget.AddToViewport` _returnvalue 0)
        (set `self.PauseWidget` _returnvalue)
        (`WidgetBlueprintLibrary.SetInputMode_UIOnlyEx` self _returnvalue)
        (set `self.bShowMouseCursor` true))
      (:`Is Not Valid`
        (`GameplayStatics.OpenLevel` "MainMenu" false)))))

(event `InputAxis|Forward`
  (params (AxisValue :type "Float (single-precision)"))
  (bind _returnvalue (`self.K2_GetPawn`))
  ;[1 1 1] Input
  (`/Engine/EditorBlueprintResources/StandardMacros.IsValid` _returnvalue
    (:`Is Valid`
      (`Pawn.AddMovementInput` _returnvalue (`self.GetActorForwardVector` _returnvalue) AxisValue false))))

(event `InputAxis|Right`
  (params (AxisValue :type "Float (single-precision)"))
  (bind _returnvalue (`self.K2_GetPawn`))
  ;[1 1 1] Input
  (`/Engine/EditorBlueprintResources/StandardMacros.IsValid` _returnvalue
    (:`Is Valid`
      (`Pawn.AddMovementInput` _returnvalue (`self.GetActorRightVector` _returnvalue) AxisValue false))))

(event `InputAxis|LookUp`
  (params (AxisValue :type "Float (single-precision)"))
  (bind _returnvalue (`self.K2_GetPawn`))
  ;[1 1 1] Input
  (`/Engine/EditorBlueprintResources/StandardMacros.IsValid` _returnvalue
    (:`Is Valid`
      (`Pawn.AddControllerPitchInput` _returnvalue AxisValue))))

(event `InputAxis|LookRight`
  (params (AxisValue :type "Float (single-precision)"))
  (bind _returnvalue (`self.K2_GetPawn`))
  ;[1 1 1] Input
  (`/Engine/EditorBlueprintResources/StandardMacros.IsValid` _returnvalue
    (:`Is Valid`
      (`Pawn.AddControllerYawInput` _returnvalue AxisValue))))

(event `InputAction|Jump`
  (params (Key :type "Key Structure"))
  (bind _returnvalue (`self.K2_GetPawn`))
  ;[1 1 1] Input
  (:`Pressed`
    (`/Engine/EditorBlueprintResources/StandardMacros.IsValid` _returnvalue
      (:`Is Valid`
        (bind _ascharacter (cast `Character` _returnvalue))
        (`Character.Jump` _ascharacter))))
  (:`Released`
    (`/Engine/EditorBlueprintResources/StandardMacros.IsValid` _returnvalue
      (:`Is Valid`
        (bind _ascharacter_2 (cast `Character` _returnvalue))
        (`Character.StopJumping` _ascharacter_2)))))

(fn `UserConstructionScript`)