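; ScreenController is a player controller that puts a menu widget on screen and switches the player to UI control.
; Its ShowMenu event creates the passed widget class, requires it to be a MainMenuUI, and fills its SeedInput with the SeedString from the MainGI game instance.
; It then adds the widget to the player screen, sets UI-only input focused on it and shows the mouse cursor.
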(event `ShowMenu`
  (params (Widget :type "UserWidget Class Reference"))
  (bind _asmain_gi (cast `/Game/Blueprints/Rules/MainGI` (`GameplayStatics.GetGameInstance`)))
  (bind _returnvalue (`|CreateWidget` Widget self))
  (bind _asmain_menu_ui (cast `/Game/UI/MainMenuUI` _returnvalue))
  (`EditableTextBox.SetText` (`/Game/UI/MainMenuUI.SeedInput` _asmain_menu_ui) (`KismetTextLibrary.Conv_StringToText` (`/Game/Blueprints/Rules/MainGI.SeedString` _asmain_gi)))
  (`UserWidget.AddToPlayerScreen` _returnvalue 0)
  (`WidgetBlueprintLibrary.SetInputMode_UIOnlyEx` self _returnvalue)
  (set `self.bShowMouseCursor` true))

(fn `UserConstructionScript`)