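; AI controller that drives a possessed VehicleTrack along its assigned Route at constant full throttle.
; Each tick, it steers toward the path's forward direction when within SufficientDistance, otherwise from the predicted location toward its nearest path point.
; Cross and dot products between heading and desired direction set steering sign and strength.
; Box-trace avoidance of other vehicles is disconnected, and the GetSteeringInput separation helper is never called.
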(event `self.ReceiveBeginPlay`)

(event `self.OnPossess`
  (params (PossessedPawn :type "Pawn Object Reference"))
  (bind _asvehicle_track (cast `/Game/Blueprints/Actors/Track/VehicleTrack` PossessedPawn))
  (set `self.Route` (`/Game/Blueprints/Actors/Track/VehicleTrack.Route` _asvehicle_track)))

(event `self.ReceiveTick`
  (params (DeltaSeconds :type "Float (single-precision)"))
  (bind _route (`self.Route`))
  (bind _path (`/Game/Blueprints/Actors/Route.Path` _route))
  (bind _asvehicle_track (cast `/Game/Blueprints/Actors/Track/VehicleTrack` (`self.K2_GetPawn`)))
  (bind _vehiclemovement (`WheeledVehicle.VehicleMovement` _asvehicle_track))
  (`WheeledVehicleMovementComponent.SetThrottleInput` _vehiclemovement 1.0)
  (`/Engine/EditorBlueprintResources/StandardMacros.IsValid` _route
    (:`Is Valid`
      (bind _returnvalue (`self.K2_GetActorLocation` _asvehicle_track))
      (bind (_returnvalue_location _returnvalue_rotation) (`KismetMathLibrary.BreakTransform` (`SplineComponent.FindTransformClosestToWorldLocation` _path _returnvalue "World" false)))
      (bind _loaction (`/Game/Blueprints/Actors/Track/VehicleTrack.PredictLocation` _asvehicle_track (`self.PredictionTime`)))
      (bind _returnvalue_location_2 (`KismetMathLibrary.BreakTransform` (`SplineComponent.FindTransformClosestToWorldLocation` _path _loaction "World" false)))
      (bind _returnvalue_2 (`KismetMathLibrary.SelectVector` (`KismetMathLibrary.GetForwardVector` _returnvalue_rotation) (`KismetMathLibrary.Normal` (- _returnvalue_location_2 _loaction)) (<= (`KismetMathLibrary.VSize` (- _returnvalue _returnvalue_location)) (`self.SufficientDistance`))))
      (bind _returnvalue_3 (`KismetMathLibrary.Normal` (- _loaction _returnvalue)))
      (bind _returnvalue_4 (`KismetMathLibrary.Cross_VectorVector` _returnvalue_2 _returnvalue_3))
      (`WheeledVehicleMovementComponent.SetSteeringInput` _vehiclemovement (`KismetMathLibrary.FClamp` (* (`KismetMathLibrary.SelectFloat` -1.0 1.0 (>= (`KismetMathLibrary.Dot_VectorVector` (`self.GetActorUpVector` _asvehicle_track) _returnvalue_4) 0.0)) (`KismetMathLibrary.SelectFloat` (`KismetMathLibrary.VSize` _returnvalue_4) 1.0 (>= (`KismetMathLibrary.Dot_VectorVector` _returnvalue_3 _returnvalue_2) 0.0))) -1.0)))))

(fn `GetSteeringInput`
  (params (Track :type "/Game/Blueprints/Actors/Track/VehicleTrack Object Reference"))
  (returns (SteeringInput :type "Float (double-precision)"))
  (locals (Steering :type "Float (double-precision)"))
  (bind _returnvalue (`self.K2_GetActorLocation` Track))
  (bind _predictiontime (`self.PredictionTime`))
  (bind _returnvalue_2 (- (`/Game/Blueprints/Actors/Track/VehicleTrack.PredictLocation` Track _predictiontime) _returnvalue))
  (bind _outactors (`GameplayStatics.GetAllActorsOfClass` "/Game/Blueprints/Actors/Track/VehicleTrack.VehicleTrack_C"))
  (for _array_element _outactors
    (bind _returnvalue_3 (- (`/Game/Blueprints/Actors/Track/VehicleTrack.PredictLocation` _array_element _predictiontime) _returnvalue))
    (bind _returnvalue_4 (`KismetMathLibrary.Dot_VectorVector` _returnvalue_2 _returnvalue_3))
    (bind _output_get (set `local.Steering` (+ (stale _output_get) (* (`KismetMathLibrary.SelectFloat` (* _returnvalue_4 (`KismetMathLibrary.SelectFloat` -1.0 1.0 (>= (`KismetMathLibrary.Dot_VectorVector` (`self.GetActorUpVector` Track) (`KismetMathLibrary.Cross_VectorVector` _returnvalue_2 _returnvalue_3)) 0.0))) 0.0 (>= _returnvalue_4 0.0)) (/ (`KismetMathLibrary.VSize` _returnvalue_3) (`KismetMathLibrary.VSize` _returnvalue_2)))))))
  (return (`KismetMathLibrary.FClamp` (`local.Steering`) -1.0)))

(fn `UserConstructionScript`)