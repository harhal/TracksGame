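; Driver is a simple autopilot controller that drives a possessed SimplePhisycTrack pawn.
; Each tick it applies full gas, then box-traces on the Visibility channel from the pawn's Head along its engine velocity, using the Cube's rotation and ignoring the pawn.
; When the look-ahead trace hits, it applies full turn input, always in the same direction, as basic obstacle avoidance.
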(event `self.ReceiveTick`
  (params (DeltaSeconds :type "Float (single-precision)"))
  (bind _assimple_phisyc_track (cast `/Game/Blueprints/SimpleTrack_Old/SimplePhisycTrack` (`self.K2_GetPawn`)))
  (`/Game/Blueprints/SimpleTrack_Old/SimplePhisycTrack.Gas` _assimple_phisyc_track 1.0 DeltaSeconds)
  (bind _returnvalue (`SceneComponent.K2_GetComponentLocation` (`/Game/Blueprints/SimpleTrack_Old/SimplePhisycTrack.Head` _assimple_phisyc_track)))
  (bind (_outhit _returnvalue_2) (`KismetSystemLibrary.BoxTraceSingle` _returnvalue (+ _returnvalue (* (`/Game/Blueprints/SimpleTrack_Old/SimplePhisycTrack.GetEngineVelocity` _assimple_phisyc_track) 3.0)) (320.0 350.0 300.0) (`SceneComponent.K2_GetComponentRotation` (`/Game/Blueprints/SimpleTrack_Old/SimplePhisycTrack.Cube` _assimple_phisyc_track)) "TraceTypeQuery1" false (`|MakeArray` _assimple_phisyc_track :!type "Actor Object Reference")))
  (if _returnvalue_2
    (`/Game/Blueprints/SimpleTrack_Old/SimplePhisycTrack.Turn` _assimple_phisyc_track 1.0 DeltaSeconds)))

(fn `UserConstructionScript`)