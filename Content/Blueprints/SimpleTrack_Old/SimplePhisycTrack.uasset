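; Simple physics vehicle prototype that drives and steers a Cube body through Gas and Turn events.
; Gas pushes the body at Head along ForwardEngine's forward vector while projected forward speed is below MaxSpeed and a debug-drawn ForwardAxle downtrace hits.
; Turn applies acceleration-based yaw torque around the Cube's up axis, without a ground check.
; The BackwardAxle trace is unconnected and Tick is empty.
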(event `Gas`
  (params (Input :type "Float (double-precision)") (DeltaSeconds :type "Float (double-precision)"))
  (bind _forwardaxle (`self.ForwardAxle`))
  (bind _returnvalue (`SceneComponent.K2_GetComponentLocation` _forwardaxle))
  ;[1 1 1] Gas
  (bind (_outhit _returnvalue_2) (`KismetSystemLibrary.LineTraceSingle` _returnvalue (+ _returnvalue (* (`SceneComponent.GetUpVector` _forwardaxle) (* (`self.ShasselHeight`) -1.0))) "TraceTypeQuery1" false (`|MakeArray` self :!type "Actor Object Reference") "ForOneFrame"))
  (if (and (< (`self.GetVeloctyProjection`) (`self.MaxSpeed`)) (or _returnvalue_2 _returnvalue_2))
    (`PrimitiveComponent.AddForceAtLocation` (`self.Cube`) (* (`SceneComponent.GetForwardVector` (`self.ForwardEngine`)) (* Input DeltaSeconds (`self.EngineForce`))) (`SceneComponent.K2_GetComponentLocation` (`self.Head`)) "None")))

(event `Turn`
  (params (Input :type "Float (double-precision)") (DeltaSeconds :type "Float (double-precision)"))
  ;[1 1 1] Turn
  (`PrimitiveComponent.AddTorqueInDegrees` (`self.Cube`) (* (`SceneComponent.GetUpVector` (`self.Cube`)) (* Input DeltaSeconds (`self.TurnForce`))) "None" true))

(event `self.ReceiveTick`
  (params (DeltaSeconds :type "Float (single-precision)")))

(fn `GetEngineVelocity`
  (returns (Velocity :type "Vector Structure"))
  (return (* (`KismetMathLibrary.Normal` (`SceneComponent.GetForwardVector` (`self.ForwardEngine`))) (`self.GetVeloctyProjection`))))

(fn `GetVeloctyProjection`
  (returns (Projection :type "Float (double-precision)"))
  (bind _returnvalue (`SceneComponent.GetForwardVector` (`self.ForwardEngine`)))
  (return (/ (`KismetMathLibrary.Dot_VectorVector` (`self.GetVelocity`) _returnvalue) (`KismetMathLibrary.VSize` _returnvalue))))

(fn `UserConstructionScript`)