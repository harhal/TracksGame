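; MainGM is the game mode that handles the end of a game and saving of results.
; EndGame passes the win flag on to the MainPC player controller.
; SaveResult fills a fresh SaveData object from the MainGI game instance through SaveGI and writes it to the HighScores slot without loading the existing save.
; ReadyToStartMatch always returns false, so the match does not start automatically.
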(event `EndGame`
  (params (Win :type Boolean))
  (bind _asmain_pc (cast `/Game/Blueprints/Controllers/MainPC` (`GameplayStatics.GetPlayerController` 0)))
  (`/Game/Blueprints/Controllers/MainPC.EndGame` _asmain_pc Win))

(event `SaveResult`
  (bind _asmain_gi (cast `/Game/Blueprints/Rules/MainGI` (`GameplayStatics.GetGameInstance`)))
  (bind _returnvalue (`GameplayStatics.CreateSaveGameObject` "/Game/Blueprints/SaveData.SaveData_C"))
  (`/Game/Blueprints/SaveData.SaveGI` _returnvalue _asmain_gi)
  (`GameplayStatics.SaveGameToSlot` _returnvalue "HighScores"))

(fn `ReadyToStartMatch`
  (returns (ReturnValue :type Boolean))
  (return false))

(fn `UserConstructionScript`)