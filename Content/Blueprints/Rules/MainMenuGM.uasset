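; Main menu game mode that loads saved high scores and opens the menu on play start.
; LoadData reads the HighScores save slot, or creates a new SaveData object when none exists, and calls its LoadGI to pass the data to the MainGI game instance.
; BeginPlay then has the ScreenController player controller show MainMenuUI.
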(event `self.ReceiveBeginPlay`
  (`self.LoadData`)
  (bind _asscreen_controller (cast `/Game/Blueprints/Controllers/ScreenController` (`GameplayStatics.GetPlayerController` 0)))
  (`/Game/Blueprints/Controllers/ScreenController.ShowMenu` _asscreen_controller "/Game/UI/MainMenuUI.MainMenuUI_C"))

(event `LoadData`
  (bind _asmain_gi (cast `/Game/Blueprints/Rules/MainGI` (`GameplayStatics.GetGameInstance`)))
  (bind _returnvalue (`GameplayStatics.LoadGameFromSlot` "HighScores"))
  (`/Engine/EditorBlueprintResources/StandardMacros.IsValid` _returnvalue
    (:`Is Valid`
      (bind _assave_data (cast `/Game/Blueprints/SaveData` _returnvalue)
        (:`then`
          (`/Game/Blueprints/SaveData.LoadGI` _assave_data _asmain_gi))
        (:`CastFailed`
          (`/Game/Blueprints/SaveData.LoadGI` (stale _returnvalue_2) _asmain_gi :!label _label))))
    (:`Is Not Valid`
      (bind _returnvalue_2 (`GameplayStatics.CreateSaveGameObject` "/Game/Blueprints/SaveData.SaveData_C"))
      (goto _label))))

(fn `UserConstructionScript`)