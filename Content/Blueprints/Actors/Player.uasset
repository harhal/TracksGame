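; Player character that spawns above a track, records achievement stats and ends the game on contact with the ground or a route.
; On possession it moves to the MainPC's SpawnTrack at a fixed height, matching the track's rotation.
; Tick and jump events accumulate game time, airborne time and jump count in MainGI.
; Hitting Ground calls MainGM EndGame(false), overlapping Route calls EndGame(true); both then disable capsule collision and destroy the MainPC-controlled pawn.
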(event `self.ReceivePossessed`
  (params (NewController :type "Controller Object Reference"))
  ;[1 1 1] Spawner
  (bind _asmain_pc (cast `/Game/Blueprints/Controllers/MainPC` NewController))
  (bind _returnvalue (`self.GetTransform` (`/Game/Blueprints/Controllers/MainPC.SpawnTrack` _asmain_pc)))
  (`self.K2_SetActorLocationAndRotation` (`KismetMathLibrary.MakeVector` (.x (.location _returnvalue)) (.y (.location _returnvalue)) 600.0) (.rotation _returnvalue)))

(event `self.ReceiveTick`
  (params (DeltaSeconds :type "Float (single-precision)"))
  ;[1 1 1] Achivement counter
  (bind _asmain_gi (cast `/Game/Blueprints/Rules/MainGI` (`GameplayStatics.GetGameInstance`)))
  (bind _output_get (set `/Game/Blueprints/Rules/MainGI.GameTime` (+ (stale _output_get) DeltaSeconds) _asmain_gi))
  (if (and (`NavMovementComponent.IsFalling` (`self.CharacterMovement`)) (`self.IsAlive`))
    (bind _output_get_2 (set `/Game/Blueprints/Rules/MainGI.FlyTime` (+ (stale _output_get_2) DeltaSeconds) _asmain_gi))))

(event `self.OnJumped`
  ;[1 1 1] Achivement counter
  (if (`self.IsAlive`)
    (bind _asmain_gi (cast `/Game/Blueprints/Rules/MainGI` (`GameplayStatics.GetGameInstance`)))
    (bind _output_get (set `/Game/Blueprints/Rules/MainGI.JumpCount` (+ (stale _output_get) 1) _asmain_gi))))

(event `self.CapsuleComponent.OnComponentHit`
  (params (HitComponent :type "PrimitiveComponent Object Reference") (OtherActor :type "Actor Object Reference") (OtherComp :type "PrimitiveComponent Object Reference") (NormalImpulse :type "Vector Structure") (Hit :type "HitResult Structure (by ref)"))
  ;[1 1 1] EndGameTrigger
  (cast `/Game/Blueprints/Actors/Ground` OtherActor)
  (`/Game/Blueprints/Rules/MainGM.EndGame` (cast `/Game/Blueprints/Rules/MainGM` (`GameplayStatics.GetGameMode`) :!pure true) false)
  (`PrimitiveComponent.SetCollisionEnabled` (`self.CapsuleComponent`) "NoCollision" :!label _label)
  (cast `/Game/Blueprints/Controllers/MainPC` (`self.GetController`))
  (`self.K2_DestroyActor`))

(event `self.CapsuleComponent.OnComponentBeginOverlap`
  (params (OverlappedComponent :type "PrimitiveComponent Object Reference") (OtherActor :type "Actor Object Reference") (OtherComp :type "PrimitiveComponent Object Reference") (OtherBodyIndex :type Integer) (bFromSweep :type Boolean) (SweepResult :type "HitResult Structure (by ref)"))
  ;[1 1 1] EndGameTrigger
  (cast `/Game/Blueprints/Actors/Route` OtherActor)
  (`/Game/Blueprints/Rules/MainGM.EndGame` (cast `/Game/Blueprints/Rules/MainGM` (`GameplayStatics.GetGameMode`) :!pure true) true)
  (goto _label))

(fn `UserConstructionScript`)